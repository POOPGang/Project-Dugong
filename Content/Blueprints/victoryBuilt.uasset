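; Actor Blueprint, apparently a built victory structure, that pushes the overworld game toward a win when it begins play.
; On BeginPlay it casts the game mode to GM_Overworld, spends one Mysterium2 and lowers DOOM by a fixed step.
; If DOOM then falls below a near-zero threshold, it creates the YOUWIN widget and adds it to the viewport.
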(event `self.ReceiveActorOnClicked`
  (params (ButtonPressed :type "Key Structure")))

(event `self.ReceiveBeginPlay`
  (bind _asgm_overworld (cast `/Game/Blueprints/GM_Overworld` (`GameplayStatics.GetGameMode`)))
  (set `/Game/Blueprints/GM_Overworld.mysterium2` (+ (`/Game/Blueprints/GM_Overworld.mysterium2` _asgm_overworld) -1) _asgm_overworld)
  (bind _output_get (set `/Game/Blueprints/GM_Overworld.DOOM` (+ (`/Game/Blueprints/GM_Overworld.DOOM` _asgm_overworld) -0.25) _asgm_overworld))
  (`/Engine/EditorBlueprintResources/StandardMacros.CompareFloat` _output_get 0.01
    (:`<`
      (bind _returnvalue (`|CreateWidget` "/Game/Blueprints/YOUWIN.YOUWIN_C"))
      (`UserWidget.AddToViewport` _returnvalue 0))))

(fn `UserConstructionScript`)