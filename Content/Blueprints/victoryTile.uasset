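; Clickable overworld tile actor, named as the victory node, that opens a build prompt when selected.
; On click it registers itself as the current node in GM_Overworld, stores its view-point location as the new ship location, then adds a BuildQu widget to the viewport.
; It contains no victory logic; disconnected leftover nodes would teleport the player pawn and increment Mysterium2, but never run.
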(event `self.ReceiveActorOnClicked`
  (params (ButtonPressed :type "Key Structure"))
  (bind _asgm_overworld (cast `/Game/Blueprints/GM_Overworld` (`GameplayStatics.GetGameMode`)))
  (set `/Game/Blueprints/GM_Overworld.curNode` self _asgm_overworld)
  (set `/Game/Blueprints/GM_Overworld.newShipLocation` (`self.GetActorEyesViewPoint`) _asgm_overworld)
  (bind _returnvalue (`|CreateWidget` "/Game/Blueprints/buildQu.buildQu_C"))
  (`UserWidget.AddToViewport` _returnvalue 0))

(fn `UserConstructionScript`)