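; Overworld game instance that saves and restores the node actors of two districts in one save slot.
; Saving records class and transform of every actor of the listed node types into that district's array, copying the other district's array from DistSave.
; Populating destroys existing nodes and respawns saved ones.
; District 1 loads from the slot, while District 2 reads the in-memory DistSave, which District 1 population resets to an empty object.
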(fn `fetchActiveNodes`
  (returns (returns :type "Array of /Game/Blueprints/Overworld/saveSpace/nodeStruct Structure"))
  (`KismetArrayLibrary.Array_Clear` (`self.savedNodes`))
  (for _array_element (`self.listOfNodeTypes`)
    (bind _outactors (`GameplayStatics.GetAllActorsOfClass` _array_element))
    (for _array_element_2 _outactors
      (`KismetArrayLibrary.Array_Add` (`self.savedNodes`) (make `/Game/Blueprints/Overworld/saveSpace/nodeStruct` _array_element (`Actor.GetTransform` _array_element_2)))))
  (return (`self.savedNodes`)))

(fn `populateDist1`
  (bind _returnvalue (`GameplayStatics.CreateSaveGameObject` "/Game/Blueprints/Overworld/saveSpace/overworldSave.overworldSave_C"))
  (set `self.distSave` _returnvalue)
  (bind _returnvalue_2 (`GameplayStatics.LoadGameFromSlot` "0"))
  (bind _asoverworld_save (cast `/Game/Blueprints/Overworld/saveSpace/overworldSave` _returnvalue_2))
  (`self.removeAllNodes`)
  (for _array_element (`/Game/Blueprints/Overworld/saveSpace/overworldSave.district1Nodes` _asoverworld_save)
    (bind (_class _transform) (break `/Game/Blueprints/Overworld/saveSpace/nodeStruct` _array_element))
    (`|SpawnActorFromClass` _class _transform "AlwaysSpawn" "OverrideRootScale" null null)))

(fn `populateDist2`
  (`self.removeAllNodes`)
  (for _array_element (`/Game/Blueprints/Overworld/saveSpace/overworldSave.district2Nodes` (`self.distSave`))
    (bind (_class _transform) (break `/Game/Blueprints/Overworld/saveSpace/nodeStruct` _array_element))
    (`|SpawnActorFromClass` _class _transform "AlwaysSpawn" "OverrideRootScale" null null)))

(fn `removeAllNodes`
  (for _array_element (`self.listOfNodeTypes`)
    (bind _outactors (`GameplayStatics.GetAllActorsOfClass` _array_element))
    (for _array_element_2 _outactors
      (`Actor.K2_DestroyActor` _array_element_2))))

(fn `saveDist1Nodes`
  (bind _output_get (set `self.otherNodes` (`/Game/Blueprints/Overworld/saveSpace/overworldSave.district2Nodes` (`self.distSave`))))
  (bind _returnvalue (`GameplayStatics.CreateSaveGameObject` "/Game/Blueprints/Overworld/saveSpace/overworldSave.overworldSave_C"))
  (bind _output_get_2 (set `self.distSave` _returnvalue))
  (bind _returns (`self.fetchActiveNodes`))
  (set `/Game/Blueprints/Overworld/saveSpace/overworldSave.district1Nodes` _returns _output_get_2)
  (set `/Game/Blueprints/Overworld/saveSpace/overworldSave.district2Nodes` _output_get _output_get_2)
  (`GameplayStatics.SaveGameToSlot` _output_get_2 "0"))

(fn `saveDist2Nodes`
  (bind _output_get (set `self.otherNodes` (`/Game/Blueprints/Overworld/saveSpace/overworldSave.district1Nodes` (`self.distSave`))))
  (bind _returnvalue (`GameplayStatics.CreateSaveGameObject` "/Game/Blueprints/Overworld/saveSpace/overworldSave.overworldSave_C"))
  (bind _output_get_2 (set `self.distSave` _returnvalue))
  (bind _returns (`self.fetchActiveNodes`))
  (set `/Game/Blueprints/Overworld/saveSpace/overworldSave.district1Nodes` _output_get _output_get_2)
  (set `/Game/Blueprints/Overworld/saveSpace/overworldSave.district2Nodes` _returns _output_get_2)
  (`GameplayStatics.SaveGameToSlot` _output_get_2 "0"))