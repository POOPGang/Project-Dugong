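; Overworld game mode that shows the HUD and Debug widgets and manages the player's resources and Doom meter.
; Up/down functions adjust Mysterium, Scrap, Energy and Doom on MasterGameInstance, with Doom rising in small steps and falling in larger ones.
; Scrap and Mysterium checks return true when positive, otherwise show a NotEnough widget, while CheckWinCondition shows YOUWIN once Doom is near zero.
; A failed game-instance cast calls TestCore, which shows an error widget.
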(event `self.ReceiveBeginPlay`
  (bind _returnvalue (`|CreateWidget` "/Game/Blueprints/Overworld/Overworld_HUD.Overworld_HUD_C"))
  (`UserWidget.AddToViewport` _returnvalue 0)
  (bind _returnvalue_2 (`|CreateWidget` "/Game/Blueprints/Overworld/debug.debug_C"))
  (`UserWidget.AddToViewport` _returnvalue_2 0))

(fn `checkMysterium`
  (returns (hasEnough :type Boolean))
  (bind _asmaster_game_instance (cast `MasterGameInstance` (`GameplayStatics.GetGameInstance`))
    (:`then`
      (`/Engine/EditorBlueprintResources/StandardMacros.CompareInt` (`MasterGameInstance.mysterium` _asmaster_game_instance)
        (:`>`
          (return true))
        (:`==`
          _)
        (:`<`
          _))
      (set `MasterGameInstance.ERROR_message` "mysterium" _asmaster_game_instance)
      (bind _returnvalue (`|CreateWidget` "/Game/Blueprints/Overworld/notEnough.notEnough_C"))
      (`UserWidget.AddToViewport` _returnvalue 0))
    (:`CastFailed`
      (`self.testCore` false))))

(fn `checkScrap`
  (returns (hasEnough :type Boolean))
  (bind _asmaster_game_instance (cast `MasterGameInstance` (`GameplayStatics.GetGameInstance`))
    (:`then`
      (`/Engine/EditorBlueprintResources/StandardMacros.CompareInt` (`MasterGameInstance.scrap` _asmaster_game_instance)
        (:`>`
          (return true))
        (:`==`
          _)
        (:`<`
          _))
      (set `MasterGameInstance.ERROR_message` "scrap" _asmaster_game_instance)
      (bind _returnvalue (`|CreateWidget` "/Game/Blueprints/Overworld/notEnough.notEnough_C"))
      (`UserWidget.AddToViewport` _returnvalue 0))
    (:`CastFailed`
      (`self.testCore` false))))

(fn `checkWinCondition`
  (bind _asmaster_game_instance (cast `MasterGameInstance` (`GameplayStatics.GetGameInstance`))
    (:`then`
      (`/Engine/EditorBlueprintResources/StandardMacros.CompareFloat` (`MasterGameInstance.DOOOM` _asmaster_game_instance) 0.01
        (:`<`
          (bind _returnvalue (`|CreateWidget` "/Game/Blueprints/Overworld/YOUWIN.YOUWIN_C"))
          (`UserWidget.AddToViewport` _returnvalue 0))))
    (:`CastFailed`
      (`self.testCore` false))))

(fn `downDoom`
  (bind _asmaster_game_instance (cast `MasterGameInstance` (`GameplayStatics.GetGameInstance`))
    (:`then`
      (set `MasterGameInstance.DOOOM` (- (`MasterGameInstance.DOOOM` _asmaster_game_instance) 0.25) _asmaster_game_instance))
    (:`CastFailed`
      (`self.testCore` false))))

(fn `downEnergy`
  (bind _asmaster_game_instance (cast `MasterGameInstance` (`GameplayStatics.GetGameInstance`))
    (:`then`
      (set `MasterGameInstance.energy` (- (`MasterGameInstance.energy` _asmaster_game_instance) 1) _asmaster_game_instance))
    (:`CastFailed`
      (`self.testCore` false))))

(fn `downMysterium`
  (bind _asmaster_game_instance (cast `MasterGameInstance` (`GameplayStatics.GetGameInstance`))
    (:`then`
      (set `MasterGameInstance.mysterium` (- (`MasterGameInstance.mysterium` _asmaster_game_instance) 1) _asmaster_game_instance))
    (:`CastFailed`
      (`self.testCore` false))))

(fn `downScrap`
  (bind _asmaster_game_instance (cast `MasterGameInstance` (`GameplayStatics.GetGameInstance`))
    (:`then`
      (set `MasterGameInstance.scrap` (- (`MasterGameInstance.scrap` _asmaster_game_instance) 1) _asmaster_game_instance))
    (:`CastFailed`
      (`self.testCore` false))))

(fn `testCore`
  (params (pass :type Boolean))
  (bind _returnvalue (`|CreateWidget` "/Game/Blueprints/Overworld/ERROR_message.ERROR_message_C"))
  (`UserWidget.AddToViewport` _returnvalue 0))

(fn `upDoom`
  (bind _asmaster_game_instance (cast `MasterGameInstance` (`GameplayStatics.GetGameInstance`))
    (:`then`
      (set `MasterGameInstance.DOOOM` (+ (`MasterGameInstance.DOOOM` _asmaster_game_instance) 0.02) _asmaster_game_instance))
    (:`CastFailed`
      (`self.testCore` false))))

(fn `upEnergy`
  (bind _asmaster_game_instance (cast `MasterGameInstance` (`GameplayStatics.GetGameInstance`))
    (:`then`
      (set `MasterGameInstance.energy` (+ (`MasterGameInstance.energy` _asmaster_game_instance) 1) _asmaster_game_instance))
    (:`CastFailed`
      (`self.testCore` false))))

(fn `upMysterium`
  (bind _asmaster_game_instance (cast `MasterGameInstance` (`GameplayStatics.GetGameInstance`))
    (:`then`
      (set `MasterGameInstance.mysterium` (+ (`MasterGameInstance.mysterium` _asmaster_game_instance) 1) _asmaster_game_instance))
    (:`CastFailed`
      (`self.testCore` false))))

(fn `upScrap`
  (bind _asmaster_game_instance (cast `MasterGameInstance` (`GameplayStatics.GetGameInstance`))
    (:`then`
      (set `MasterGameInstance.scrap` (+ (`MasterGameInstance.scrap` _asmaster_game_instance) 1) _asmaster_game_instance))
    (:`CastFailed`
      (`self.testCore` false))))

(fn `UserConstructionScript`)