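; Underworld player controller that handles mouse input for selecting units and ordering moves on tiles.
; Both buttons trace from the cursor against one object type; left click, on the player's turn only, selects the hit BaseUnit or clears the active unit and tile.
; Right click has no turn check; it clicks the hit BaseTile, then has the active unit's AI controller move, subject to a moving and action-point check.
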(event `Key|LeftMouseButton`
  (params (Key :type "Key Structure"))
  (bind (_worldlocation _worlddirection) (`self.DeprojectMousePositionToWorld` (`GameplayStatics.GetPlayerController` 0)))
  ;[1 1 1] Unit Selection
  ;;[1 1 1] Decide whether to process input based on game state
  (:`Pressed`
    (bind _asunderworld_game_state (cast `UnderworldGameState` (`GameplayStatics.GetGameState`))
      (:`then`
        (bind _returnvalue (`UnderworldGameState.GetIsPlayerTurn` _asunderworld_game_state))
        (if _returnvalue
          ;;[1 1 1] Line Trace Results
          (bind (_outhit _returnvalue_2) (`KismetSystemLibrary.LineTraceSingleForObjects` _worldlocation (+ _worldlocation (* (`KismetMathLibrary.GetForwardVector` (`KismetMathLibrary.Conv_VectorToRotator` _worlddirection)) 10000000.0)) (`|MakeArray` "ObjectTypeQuery7" :!type "EObjectTypeQuery Enum")))
          (if _returnvalue_2
            (bind _asbase_unit (cast `BaseUnit` (`.HitActor` (`GameplayStatics.BreakHitResult` _outhit)))
              (:`then`
                (`BaseUnit.UnitOnClicked` :`self` _asbase_unit))
              (:`CastFailed`
                ;;[1 1 1] Clear unit and tile on left click on non-unit
                (bind _asunderworld_game_state_2 (cast `UnderworldGameState` (`GameplayStatics.GetGameState`) :!label _label))
                (`UnderworldGameState.ClearActiveUnit` _asunderworld_game_state_2)
                (`UnderworldGameState.ClearActiveTile` _asunderworld_game_state_2)))
            (else
              (goto _label)))))
      (:`CastFailed`
        (`KismetSystemLibrary.PrintString` "Error: Underworld Game State not found")))))

(event `Key|RightMouseButton`
  (params (Key :type "Key Structure"))
  (bind (_worldlocation _worlddirection) (`self.DeprojectMousePositionToWorld` (`GameplayStatics.GetPlayerController` 0)))
  (:`Pressed`
    (bind _asunderworld_game_state (cast `UnderworldGameState` (`GameplayStatics.GetGameState`))
      (:`then`
        ;[1 1 1] Line Trace Results
        (bind (_outhit _returnvalue) (`KismetSystemLibrary.LineTraceSingleForObjects` _worldlocation (+ _worldlocation (* (`KismetMathLibrary.GetForwardVector` (`KismetMathLibrary.Conv_VectorToRotator` _worlddirection)) 10000000.0)) (`|MakeArray` "ObjectTypeQuery7" :!type "EObjectTypeQuery Enum")))
        (if _returnvalue
          (bind _asbase_tile (cast `BaseTile` (`.HitActor` (`GameplayStatics.BreakHitResult` _outhit))))
          (`BaseTile.TileOnClicked` :`self` _asbase_tile)
          (bind _returnvalue_2 (`UnderworldGameState.GetActiveUnit` _asunderworld_game_state))
          (`/Engine/EditorBlueprintResources/StandardMacros.IsValid` _returnvalue_2
            (:`Is Valid`
              (bind _returnvalue_3 (`BaseUnit.GetIsMoving` _returnvalue_2))
              (bind _returnvalue_4 (`BaseUnit.GetActionPoints` _returnvalue_2))
              (if (and _returnvalue_3 (> _returnvalue_4 0))
                (`KismetSystemLibrary.PrintString` "Unit movement command invalid")
                (else
                  (bind _asunderworld_unit_controller_bp (cast `/Game/Blueprints/Underworld/UnderworldUnitController_BP` (`AIBlueprintHelperLibrary.GetAIController` _returnvalue_2)))
                  (`/Game/Blueprints/Underworld/UnderworldUnitController_BP.MoveToTile` _asunderworld_unit_controller_bp)))))))
      (:`CastFailed`
        (`KismetSystemLibrary.PrintString` "Error: Underworld Game State not found")))))

(fn `UserConstructionScript`)