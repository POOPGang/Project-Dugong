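; Underworld unit controller Blueprint that moves the active unit to the active tile in what appears to be turn-based tile play.
; MoveToTile reads the active unit and tile from UnderworldGameState and proceeds only if the unit has action points and StartMoving accepts the tile.
; AI MoveTo then walks the unit to the tile actor, and StopMoving is called only when the move succeeds.
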(event `MoveToTile`
  (bind _asunderworld_game_state (cast `UnderworldGameState` (`GameplayStatics.GetGameState`)))
  (bind _returnvalue (`UnderworldGameState.GetActiveUnit` _asunderworld_game_state))
  (bind _returnvalue_2 (`UnderworldGameState.GetActiveTile` _asunderworld_game_state))
  (bind _returnvalue_3 (`BaseUnit.GetActionPoints` _returnvalue))
  (if (> _returnvalue_3 0)
    (bind _returnvalue_4 (`BaseUnit.StartMoving` _returnvalue _returnvalue_2))
    (if _returnvalue_4
      (`|AIMoveTo` _returnvalue (0.0 0.0 0.0) _returnvalue_2 0.0
        (:`OnSuccess`
          (`BaseUnit.StopMoving` _returnvalue))))))

(fn `UserConstructionScript`)