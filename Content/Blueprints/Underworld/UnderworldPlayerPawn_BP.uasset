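; Player pawn for the Underworld that flies freely under axis input and turns in fixed yaw steps.
; Pan axes sweep it along its right and forward vectors, while a vertical axis moves it in world Z within a clamped height range, all scaled by MovementSpeed and frame time.
; Clockwise and counter-clockwise actions snap yaw by 45 degrees, so panning follows the new facing.
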(event `self.ReceiveTick`
  (params (DeltaSeconds :type "Float (single-precision)")))

(event `InputAxis|PanLR`
  (params (AxisValue :type "Float (single-precision)"))
  (`self.K2_SetActorLocation` (+ (* (`self.GetActorRightVector`) (* (`self.MovementSpeed`) (* AxisValue (`GameplayStatics.GetWorldDeltaSeconds`)))) (`self.K2_GetActorLocation`)) true))

(event `InputAxis|PanFB`
  (params (AxisValue :type "Float (single-precision)"))
  (`self.K2_SetActorLocation` (+ (* (`self.GetActorForwardVector`) (* (`self.MovementSpeed`) (* AxisValue (`GameplayStatics.GetWorldDeltaSeconds`)))) (`self.K2_GetActorLocation`)) true))

(event `InputAxis|FanUD`
  (params (AxisValue :type "Float (single-precision)"))
  (`self.K2_SetActorLocation` (`KismetMathLibrary.MakeVector` (.x (`self.K2_GetActorLocation`)) (.y (`self.K2_GetActorLocation`)) (`KismetMathLibrary.FClamp` (+ (* (`self.MovementSpeed`) (* AxisValue (`GameplayStatics.GetWorldDeltaSeconds`))) (.z (`self.K2_GetActorLocation`))) 200.0 10000.0)) true))

(event `InputAction|RotateCW`
  (params (Key :type "Key Structure"))
  (:`Pressed`
    (`self.K2_SetActorRotation` (`KismetMathLibrary.MakeRotator` (.roll (`self.K2_GetActorRotation`)) (.pitch (`self.K2_GetActorRotation`)) (+ 45.0 (.yaw (`self.K2_GetActorRotation`)))))))

(event `InputAction|RotateCCW`
  (params (Key :type "Key Structure"))
  (:`Pressed`
    (`self.K2_SetActorRotation` (`KismetMathLibrary.MakeRotator` (.roll (`self.K2_GetActorRotation`)) (.pitch (`self.K2_GetActorRotation`)) (+ -45.0 (.yaw (`self.K2_GetActorRotation`)))))))

(fn `UserConstructionScript`)