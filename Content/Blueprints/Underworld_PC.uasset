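; Underworld player controller Blueprint that handles left-click selection of units in the world.
; On click, it deprojects the mouse position and line-traces a single object type along that ray, calling UnitOnClicked on any BaseUnit hit.
; It first requires an UnderworldGameState, printing an error otherwise.
; Clearing the active unit on a missed click is not connected, pending a GameInstance migration.
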(event `Key|LeftMouseButton`
  (params (Key :type "Key Structure"))
  (bind (_worldlocation _worlddirection) (`self.DeprojectMousePositionToWorld` (`GameplayStatics.GetPlayerController` 0)))
  (:`Pressed`
    (cast `UnderworldGameState` (`GameplayStatics.GetGameState`)
      (:`then`
        (if true
          ;[1 1 1] Line Trace Results
          (bind (_outhit _returnvalue) (`KismetSystemLibrary.LineTraceSingleForObjects` _worldlocation (+ _worldlocation (* (`KismetMathLibrary.GetForwardVector` (`KismetMathLibrary.Conv_VectorToRotator` _worlddirection)) 10000000.0)) (`|MakeArray` "ObjectTypeQuery7" :!type "EObjectTypeQuery Enum")))
          (if _returnvalue
            (bind _asbase_unit (cast `BaseUnit` (`.HitActor` (`GameplayStatics.BreakHitResult` _outhit))))
            (`BaseUnit.UnitOnClicked` :`self` _asbase_unit)
            (else
              ;[1 1 1] Hook up after GameInstance Migration
              (cast `UnderworldGameState` (`GameplayStatics.GetGameState`))))))
      (:`CastFailed`
        (`KismetSystemLibrary.PrintString` "Error: Underworld Game State not found")))))

(fn `UserConstructionScript`)